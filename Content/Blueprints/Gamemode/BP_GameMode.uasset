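; Game mode Blueprint that displays the player's health, armor and stamina through a test stats widget.
; BeginPlay creates the widget for player 0, adds it to the viewport, and casts the controlled pawn to BaseCharacter, printing a message on failure.
; Tick polls that character's AttributeComponent every frame and copies current values into the widget's variables, without checking that the cast succeeded.
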(event EventBeginPlay
  (bind _returnvalue (Game|GetPlayerController 0))
  (Utilities|FlowControl|Sequence
    (:then_0
      (bind _returnvalue_2 (UserInterface|CreateWidget "/Game/Blueprints/BP_WidgetTESTSTAT.BP_WidgetTESTSTAT_C" _returnvalue))
      (UserInterface|Viewport|AddtoViewport _returnvalue_2 0))
    (:then_1
      (bind _asbase_character (Utilities|Casting|CastToBaseCharacter (Pawn|GetControlledPawn _returnvalue))
        (:CastFailed
          (Development|PrintText "cast failed"))))))

(event EventTick
  (params (DeltaSeconds :type Float%20%28single-precision%29))
  (Utilities|FlowControl|Sequence
    (:then_0
      (bind _returnvalue (Class|AttributeComponent|GetCurrentHealth (Actor|GetComponentbyClass (stale EventBeginPlay _asbase_character) "/Script/Tron.AttributeComponent")))
      (Variables|/Game/Blueprints/BP_WidgetTESTSTAT.BP_WidgetTESTSTAT_C|SetHealth (stale EventBeginPlay _returnvalue_2) _returnvalue))
    (:then_1
      (bind _returnvalue_2 (Class|AttributeComponent|GetCurrentArmor (Actor|GetComponentbyClass (stale EventBeginPlay _asbase_character) "/Script/Tron.AttributeComponent")))
      (Variables|/Game/Blueprints/BP_WidgetTESTSTAT.BP_WidgetTESTSTAT_C|SetArmor (stale EventBeginPlay _returnvalue_2) _returnvalue_2))
    (:then_2
      (bind _returnvalue_3 (Class|AttributeComponent|GetCurrentStamina (Actor|GetComponentbyClass (stale EventBeginPlay _asbase_character) "/Script/Tron.AttributeComponent")))
      (Variables|/Game/Blueprints/BP_WidgetTESTSTAT.BP_WidgetTESTSTAT_C|SetStamina (stale EventBeginPlay _returnvalue_2) _returnvalue_3))))

(fn ConstructionScript)